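; Pinball flipper Blueprint that serves as either a left or right flipper, based on FlipType.
; The Construction Script derives mirrored start and end rotations from the type, sets the resting rotation, and flips X scale for the right side.
; Flip swings the Flipper component to its end rotation over FlipTime with a side-specific 2D sound.
; Flop silently returns it to the start rotation.
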(event Custom|Flip
  (Components|MoveComponentTo (Variables|Default|GetFlipper) "0, 0, 0" (Variables|Default|GetEndRotation) false false (Variables|Default|GetFlipTime) false)
  (if (Utilities|Enum|Equal(Enum) (Variables|Default|GetFlipType) "NewEnumerator0")
    (Audio|SpawnSound2D "/Game/Sounds/Cues/Pinball_FlipperLeft_Cue.Pinball_FlipperLeft_Cue" 0.1 1.0 0.0 0)
    (else
      (Audio|SpawnSound2D "/Game/Sounds/Cues/Pinball_FlipperRight_Cue.Pinball_FlipperRight_Cue" 0.1 1.0 0.0 0))))

(event Custom|Flop
  (Components|MoveComponentTo (Variables|Default|GetFlipper) "0, 0, 0" (Variables|Default|GetStartRotation) false false (Variables|Default|GetFlipTime) false))

(event EventBeginPlay)

(event Collision|EventActorBeginOverlap
  (params (OtherActor :type Actor%20Object%20Reference)))

(event EventTick
  (params (DeltaSeconds :type Float%20%28single-precision%29)))

(fn ConstructionScript
  (Variables|Default|SetStartRotation (Utilities|Select :Index (Variables|Default|GetFlipType) :NewEnumerator0 "0,25.000000, 0" :NewEnumerator1 "0,-25.000000, 0"))
  (Variables|Default|SetEndRotation (Utilities|Select :Index (Variables|Default|GetFlipType) :NewEnumerator0 "0,-25.000000, 0" :NewEnumerator1 "0,25.000000, 0"))
  (Transformation|SetRelativeRotation (Variables|Default|GetFlipper) (Variables|Default|GetStartRotation) false false)
  (switch Utilities|FlowControl|Switch|SwitchonFlipType (Variables|Default|GetFlipType)
    (:NewEnumerator1
      (Transformation|SetRelativeScale3D (Variables|Default|GetFlipper) "-1.000000,1.000000,1.000000"))))
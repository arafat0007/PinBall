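; BP_FreeMovementZone is a zone actor that adjusts the velocity of BP_Ball actors overlapping it, relative to its Arrow component.
; Each Tick, it converts ball velocity into Arrow space and uses VInterpTo toward a target with clamped, always-positive forward X and zero Y and Z.
; The result returns to world space and replaces the ball's physics linear velocity.
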(event EventBeginPlay)

(event Collision|EventActorBeginOverlap
  (params (OtherActor :type Actor%20Object%20Reference)))

(event EventTick
  (params (DeltaSeconds :type Float%20%28single-precision%29))
  (for _array_element (Collision|GetOverlappingActors "/Game/Blueprints/BP_Ball.BP_Ball_C" :!class /Script/Engine.Actor)
    (bind _asbp_ball (Utilities|Casting|CastToBP_Ball _array_element))
    (Physics|SetPhysicsLinearVelocity (Variables|/Game/Blueprints/BP_Ball.BP_Ball_C|GetBall _asbp_ball) (Math|Transform|TransformDirection (Transformation|GetWorldTransform (Variables|Default|GetArrow)) (Math|Interpolation|VInterpTo (Math|Transform|InverseTransformDirection (Transformation|GetWorldTransform (Variables|Default|GetArrow)) (Transformation|GetVelocity _array_element)) (Math|Vector|MakeVector (Math|Float|Clamp(Float) (.X (Math|Vector|BreakVector (Math|Transform|InverseTransformDirection (Transformation|GetWorldTransform (Variables|Default|GetArrow)) (Transformation|GetVelocity _array_element)))) 2e+03 4e+04) 0.0 0.0) 0.0 1.0)) false "None")))

(fn ConstructionScript)